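; BP_SwapTrigger is a trigger box that makes paired players swap body roles and control, once per team.
; On server-side overlap by a PlayerCharacter, it records the team number in ExecutedTeamIDs to block repeats.
; It finds the partner's BRPlayerState in the GameState PlayerArray via ConnectedPlayerIndex, inverts both IsLowerBody roles, then calls SwapControlWithPartner, with debug prints along the way.
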(event `self.Box.OnComponentBeginOverlap`
  (params (OverlappedComponent :type "PrimitiveComponent Object Reference") (OtherActor :type "Actor Object Reference") (OtherComp :type "PrimitiveComponent Object Reference") (OtherBodyIndex :type Integer) (bFromSweep :type Boolean) (SweepResult :type "HitResult Structure (by ref)"))
  (bind _partnerps (`self.PartnerPS`))
  (bind _executedteamids (`self.ExecutedTeamIDs`))
  (bind _myps (`self.MyPS`))
  (`/Engine/EditorBlueprintResources/ActorMacros.Switch Has Authority`
    (:`Authority`
      (bind _asplayer_character (cast `PlayerCharacter` OtherActor))
      (bind _asbrplayer_state (cast `BRPlayerState` (`Pawn.PlayerState` _asplayer_character)))
      (bind _output_get (set `self.MyPS` _asbrplayer_state))
      (bind _teamnumber (`BRPlayerState.TeamNumber` _output_get))
      (`KismetSystemLibrary.PrintString` (`KismetStringLibrary.Conv_IntToString` _teamnumber))
      (if (not (`KismetArrayLibrary.Array_Contains` _executedteamids _teamnumber))
        (`KismetArrayLibrary.Array_AddUnique` _executedteamids _teamnumber)
        (bind _returnvalue (`BRWidgetFunctionLibrary.GetBRGameState`))
        (bind _asbrplayer_state_2 (cast `BRPlayerState` (`|GetArrayItem` (`GameStateBase.PlayerArray` _returnvalue) (`BRPlayerState.ConnectedPlayerIndex` (`self.MyPS`)))))
        (bind _output_get_2 (set `self.PartnerPS` _asbrplayer_state_2))
        (set `self.NewRole_Me` (not (`BRPlayerState.bIsLowerBody` (`self.MyPS`))))
        (set `self.NewRole_Partner` (not (`BRPlayerState.bIsLowerBody` _output_get_2)))
        (`BRPlayerState.SetPlayerRole` _myps (`self.NewRole_Me`) (`BRPlayerState.ConnectedPlayerIndex` _myps))
        (`BRPlayerState.SetPlayerRole` _partnerps (`self.NewRole_Partner`) (`BRPlayerState.ConnectedPlayerIndex` _partnerps))
        (`BRPlayerState.SwapControlWithPartner` (`self.MyPS`))
        (`KismetSystemLibrary.PrintString` "Swap")))))

(fn `UserConstructionScript`)