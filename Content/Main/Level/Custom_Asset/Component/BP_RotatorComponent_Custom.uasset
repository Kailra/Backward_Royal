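; BP_RotatorComponent_Custom is a component that spins in world space around a configurable axis when auto-activated, after a fixed or randomized delay.
; A looping timer replaces Tick, adding rotation each update through a lerp weighted by the update interval and smoothing factor.
; In periodic mode, a second timer reverses velocity each period, and its elapsed fraction samples an optional curve that scales the speed.
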(event `self.ReceiveBeginPlay`
  (if (`self.bAutoActivate`)
    (`KismetSystemLibrary.Delay` (`KismetMathLibrary.SelectFloat` (`KismetMathLibrary.RandomFloatInRange` 0.0 (`self.InitialDelay`)) (`self.InitialDelay`) (`self.IsRandomRotation`)))
    (if (`self.Periodic`)
      (`KismetSystemLibrary.K2_SetTimerDelegate` (`|CreateDelegate` :!event `PeriodRotationTick`) (`self.UpdateTick`) true)
      (bind _returnvalue (`KismetSystemLibrary.K2_SetTimerDelegate` (`|CreateDelegate` :!event `OnPeriodEnded`) (`self.Period`) true))
      (set `self.PeriodTimer` _returnvalue)
      (else
        (`KismetSystemLibrary.K2_SetTimerDelegate` (`|CreateDelegate` :!event `CommonRotationTick`) (`self.UpdateTick`) true)))))

(event `CommonRotationTick`
  (`self.AddRotationByVelocity` (`self.Velocity`)))

(event `PeriodRotationTick`
  (`self.AddRotationByVelocity` (`self.GetPeriodicVelocity`)))

(event `OnPeriodEnded`
  (set `self.Velocity` (* (`self.Velocity`) -1.0)))

(event `AddRotationByVelocity`
  (params (Velocity :type "Float (double-precision)"))
  (bind _returnvalue (`self.K2_GetComponentRotation`))
  (bind (_returnvalue_x _returnvalue_y _returnvalue_z) (`KismetMathLibrary.BreakVector` (* (`self.Axis`) Velocity)))
  (`self.K2_SetWorldRotation` (`KismetMathLibrary.RLerp` (`KismetMathLibrary.ComposeRotators` (`KismetMathLibrary.MakeRotator` _returnvalue_x _returnvalue_y _returnvalue_z) _returnvalue) _returnvalue (* (`self.UpdateTick`) (`self.Smooth`)))))

(fn `GetPeriodicVelocity`
  (returns (Velocity :type "Float (double-precision)"))
  (`/Engine/EditorBlueprintResources/StandardMacros.IsValid` (`self.AdditiveCurve`)
    (:`Is Valid`
      (return (* (`CurveFloat.GetFloatValue` (`self.AdditiveCurve`) (/ (`KismetSystemLibrary.K2_GetTimerElapsedTimeHandle` (`self.PeriodTimer`)) (`self.Period`))) (`self.Velocity`))))
    (:`Is Not Valid`
      (return (`self.Velocity`)))))