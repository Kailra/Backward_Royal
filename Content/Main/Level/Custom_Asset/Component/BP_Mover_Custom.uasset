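; BP_Mover_Custom is a mover Blueprint that slides a Target from a Start offset to an End offset with configurable easing.
; BeginPlay stores the Target's initial world location as the origin for both offsets.
; On authority only, OnUpdate eases by GetAlpha and sets the location without sweep, or clears the timer once IsMoving is false.
; OnPeriodEnd clears IsMoving, and a Start/End swap is left unconnected.
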(event `self.ReceiveBeginPlay`
  (`parent.ReceiveBeginPlay`)
  (set `self.InitialLocation` (`self.K2_GetComponentLocation` (`self.Target`))))

(event `self.OnUpdate`
  (`/Engine/EditorBlueprintResources/ActorComponentMacros.Switch Has Authority`
    (:`Authority`
      (if (`self.IsMoving`)
        (`self.K2_SetWorldLocation` (`self.Target`) (+ (`|EaseFunction` (`self.Function`) (`self.GetAlpha`) (`self.Start`) (`self.End`) (`self.Exponent`)) (`self.InitialLocation`)) false false)
        (else
          (`KismetSystemLibrary.K2_ClearAndInvalidateTimerHandle` (`self.MyTimerHandle`)))))))

(event `self.OnPeriodEnd`
  (set `self.IsMoving` false))