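; BP_DeformatorBase_Custom is a base component for periodic deformation of either itself or its owner's root component.
; On BeginPlay it picks that target, optionally waits RandomInitialDelay (unrandomized), then starts looping update and period timers.
; OnPeriodEnd toggles IsReversed for back-and-forth motion, and GetAlpha returns the period's remaining-time fraction, running from 1 to 0.
; OnUpdate is empty here, so the base applies no deformation itself.
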(event `self.ReceiveBeginPlay`
  (set `self.Target` (select `bool` (`self.ApplyToSefl`) :`false` (`Actor.RootComponent` (`self.GetOwner`)) :`true` self :!type "SceneComponent Object Reference"))
  (if (`self.UseRandomInitiaslDelay`)
    (`KismetSystemLibrary.Delay` (`self.RandomInitialDelay`)))
  (`KismetSystemLibrary.K2_SetTimerDelegate` (`|CreateDelegate` :!event `OnUpdate`) (`self.UpdateTime`) true)
  (bind _returnvalue (`KismetSystemLibrary.K2_SetTimerDelegate` (`|CreateDelegate` :!event `OnPeriodEnd`) (`self.Period`) true))
  (set `self.PeriodTimer` _returnvalue))

(fn `GetAlpha`
  (returns (Result :type "Float (double-precision)"))
  (return (/ (`KismetSystemLibrary.K2_GetTimerRemainingTimeHandle` (`self.PeriodTimer`)) (`self.Period`))))

(fn `OnPeriodEnd`
  (set `self.IsReversed` (not (`self.IsReversed`))))

(fn `OnUpdate`)