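; Door obstacle with a left and a right door, one of which is randomly made passable by disabling its collision.
; On BeginPlay the authority picks a random Seed, whose RepNotify builds a random stream to choose the door.
; Replicating only the seed lets each machine derive the same choice without replicating collision state.
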(event `self.ReceiveBeginPlay`
  (`/Engine/EditorBlueprintResources/ActorMacros.Switch Has Authority`
    (:`Authority`
      (set `self.Seed` (`KismetMathLibrary.RandomInteger` 999999)))))

(fn `OnRep_Seed`
  (if (`KismetMathLibrary.RandomBoolFromStream` (`KismetMathLibrary.MakeRandomStream` (`self.Seed`)))
    (`PrimitiveComponent.SetCollisionEnabled` (`self.Door_Left`) "NoCollision")
    (else
      (`PrimitiveComponent.SetCollisionEnabled` (`self.Door_Right`) "NoCollision"))))

(fn `UserConstructionScript`)