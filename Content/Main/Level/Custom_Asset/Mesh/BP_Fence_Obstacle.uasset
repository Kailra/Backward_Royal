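; BP_Fence_Obstacle is a fence obstacle that builds rows of instanced fence meshes, each row with one randomly placed gap.
; On BeginPlay the authority picks a random Seed, whose RepNotify clears and rebuilds the instances.
; A random stream from that seed chooses each row's hole, so the same layout is generated from one replicated integer instead of replicating individual pieces.
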(event `self.ReceiveBeginPlay`
  (`/Engine/EditorBlueprintResources/ActorMacros.Switch Has Authority`
    (:`Authority`
      (set `self.Seed` (`KismetMathLibrary.RandomInteger` 999999)))))

(fn `OnRep_Seed`
  (`InstancedStaticMeshComponent.ClearInstances` (`self.InstancedStaticMesh`))
  (set `self.Stream` (`KismetMathLibrary.MakeRandomStream` (`self.Seed`)))
  (for _index (range 1 (+ (`self.RowCount`) 1))
    (bind _output_get (set `self.HoleIndex` (`KismetMathLibrary.RandomIntegerInRangeFromStream` (`self.Stream`) 1 (`self.FenceCount`))))
    (for _index_2 (range 1 (+ (`self.FenceCount`) 1))
      (if (not (== _index_2 _output_get))
        (`InstancedStaticMeshComponent.AddInstance` (`self.InstancedStaticMesh`) (`KismetMathLibrary.MakeTransform` (`KismetMathLibrary.MakeVector` (* _index (`self.RowDistance`)) (* _index_2 (`self.FenceWidth`))) (struct :`Yaw` 90.0)) false)))))

(fn `UserConstructionScript`)