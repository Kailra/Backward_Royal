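; BP_ItemSpawner is a server-authoritative spawner that periodically places random weapons and switch orbs in the level.
; On BeginPlay it starts looping timers for early weapons, late weapons and orbs.
; Early waves increment a counter until a phase threshold, after which late waves take over and clear the early timer.
; Spawn points are picked randomly from ExternalTransforms, falling back to actors tagged for each spawn type.
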(event `self.ReceiveBeginPlay`
  (`/Engine/EditorBlueprintResources/ActorMacros.Switch Has Authority`
    (:`Authority`
      (bind _returnvalue (`KismetSystemLibrary.K2_SetTimer` null "WeaponSpawn_Early" (`self.WeaponRespawn`) true))
      (set `self.EarlyTimerHandle` _returnvalue)
      (`KismetSystemLibrary.K2_SetTimer` null "WeaponSpawn_Late" (`self.WeaponRespawn`) true)
      (`KismetSystemLibrary.K2_SetTimer` null "SwitchorbSpawn" (`self.SwitchorbRespawn`) true))))

(fn `SwitchorbSpawn`
  (if (> (`KismetArrayLibrary.Array_Length` (`self.ExternalTransforms`)) 0)
    (`|SpawnActorFromClass` "/Game/Main/Item/BP_SwitchOrb.BP_SwitchOrb_C" (`KismetArrayLibrary.Array_Random` (`self.ExternalTransforms`)) "Undefined" "MultiplyWithRoot" null null)
    (else
      (bind _outactors (`GameplayStatics.GetAllActorsWithTag` "SwitchorbSpawn"))
      (`|SpawnActorFromClass` "/Game/Main/Item/BP_SwitchOrb.BP_SwitchOrb_C" (`self.GetTransform` (`KismetArrayLibrary.Array_Random` _outactors)) "Undefined" "MultiplyWithRoot" null null))))

(fn `UserConstructionScript`)

(fn `WeaponSpawn_Early`
  (if (< (`self.SpawnCount`) (`self.PhaseThreshold`))
    (set `self.SpawnCount` (+ (`self.SpawnCount`) 1))
    (for _ (range 1 (+ (`self.SpawnAmount`) 1))
      (if (> (`KismetArrayLibrary.Array_Length` (`self.ExternalTransforms`)) 0)
        (`|SpawnActorFromClass` "/Game/Main/Level/Custom_Asset/Mesh/BP_RandomWeapon.BP_RandomWeapon_C" (`KismetArrayLibrary.Array_Random` (`self.ExternalTransforms`)) "Undefined" "MultiplyWithRoot" null null)
        (else
          (bind _outactors (`GameplayStatics.GetAllActorsWithTag` "WeaponSpawn_Early"))
          (`|SpawnActorFromClass` "/Game/Main/Level/Custom_Asset/Mesh/BP_RandomWeapon.BP_RandomWeapon_C" (`self.GetTransform` (`KismetArrayLibrary.Array_Random` _outactors)) "Undefined" "MultiplyWithRoot" null null))))))

(fn `WeaponSpawn_Late`
  (if (>= (`self.SpawnCount`) (`self.PhaseThreshold`))
    (`KismetSystemLibrary.K2_ClearAndInvalidateTimerHandle` (`self.EarlyTimerHandle`))
    (for _ (range 1 (+ (`self.SpawnAmount`) 1))
      (if (> (`KismetArrayLibrary.Array_Length` (`self.ExternalTransforms`)) 0)
        (`|SpawnActorFromClass` "/Game/Main/Level/Custom_Asset/Mesh/BP_RandomWeapon.BP_RandomWeapon_C" (`KismetArrayLibrary.Array_Random` (`self.ExternalTransforms`)) "Undefined" "MultiplyWithRoot" null null)
        (else
          (bind _outactors (`GameplayStatics.GetAllActorsWithTag` "WeaponSpawn_Late"))
          (`|SpawnActorFromClass` "/Game/Main/Level/Custom_Asset/Mesh/BP_RandomWeapon.BP_RandomWeapon_C" (`self.GetTransform` (`KismetArrayLibrary.Array_Random` _outactors)) "Undefined" "MultiplyWithRoot" null null))))))