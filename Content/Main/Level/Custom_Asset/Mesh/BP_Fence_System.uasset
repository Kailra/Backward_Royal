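; Construction-script fence builder that lays a rectangular perimeter of instanced static meshes sized by Width and Depth.
; On each construction it clears the instances, then MakeWidth and MakeDepth place local-space pieces at Spacing intervals shifted by Offset, turning the Depth sides 90 degrees.
; Each opposite-side loop is nested inside the near-side loop, so those far-side instances are stacked repeatedly at the same positions.
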(fn `MakeDepth`
  (bind _spacing (`self.Spacing`))
  (bind _spacing_2 (`self.Spacing`))
  (for _index (range (`KismetMathLibrary.FTrunc` (/ (`self.Depth`) _spacing)))
    (`InstancedStaticMeshComponent.AddInstance` (`self.InstancedStaticMesh`) (`KismetMathLibrary.MakeTransform` (`KismetMathLibrary.MakeVector` 0.0 (+ (* _index _spacing) (`self.Offset`))) (struct :`Yaw` 90.0)) false)
    (for _index_2 (range (`KismetMathLibrary.FTrunc` (/ (`self.Depth`) _spacing_2)))
      (`InstancedStaticMeshComponent.AddInstance` (`self.InstancedStaticMesh`) (`KismetMathLibrary.MakeTransform` (`KismetMathLibrary.MakeVector` (`self.Width`) (+ (* _index_2 _spacing_2) (`self.Offset`))) (struct :`Yaw` 90.0)) false))))

(fn `MakeWidth`
  (bind _spacing (`self.Spacing`))
  (bind _spacing_2 (`self.Spacing`))
  (for _index (range (`KismetMathLibrary.FTrunc` (/ (`self.Width`) _spacing)))
    (`InstancedStaticMeshComponent.AddInstance` (`self.InstancedStaticMesh`) (`KismetMathLibrary.MakeTransform` (`KismetMathLibrary.MakeVector` (+ (* _index _spacing) (`self.Offset`)))) false)
    (for _index_2 (range (`KismetMathLibrary.FTrunc` (/ (`self.Width`) _spacing_2)))
      (`InstancedStaticMeshComponent.AddInstance` (`self.InstancedStaticMesh`) (`KismetMathLibrary.MakeTransform` (`KismetMathLibrary.MakeVector` (+ (* _index_2 _spacing_2) (`self.Offset`)) (`self.Depth`))) false))))

(fn `UserConstructionScript`
  (`InstancedStaticMeshComponent.ClearInstances` (`self.InstancedStaticMesh`))
  (`self.MakeWidth`)
  (`self.MakeDepth`))