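; BP_Rotator_Obstacle is a level obstacle that knocks characters away when they touch either of its two sides.
; Overlaps on Left_Collision and Right_Collision call matching launch functions, which ignore anything that is not a Character.
; Each function launches the character at a fixed speed along the direction from its Left or Right component to the character, overriding existing velocity.
; The graphs contain no rotation logic, despite the asset's name.
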(event `self.Left_Collision.OnComponentBeginOverlap`
  (params (OverlappedComponent :type "PrimitiveComponent Object Reference") (OtherActor :type "Actor Object Reference") (OtherComp :type "PrimitiveComponent Object Reference") (OtherBodyIndex :type Integer) (bFromSweep :type Boolean) (SweepResult :type "HitResult Structure (by ref)"))
  (`self.LeftLaunchPlayer` OtherActor))

(event `self.Right_Collision.OnComponentBeginOverlap`
  (params (OverlappedComponent :type "PrimitiveComponent Object Reference") (OtherActor :type "Actor Object Reference") (OtherComp :type "PrimitiveComponent Object Reference") (OtherBodyIndex :type Integer) (bFromSweep :type Boolean) (SweepResult :type "HitResult Structure (by ref)"))
  (`self.RightLaunchPlayer` OtherActor))

(fn `LeftLaunchPlayer`
  (params (Object :type "Object Object Reference"))
  (bind _ascharacter (cast `Character` Object))
  (`Character.LaunchCharacter` _ascharacter (* (`KismetMathLibrary.Normal` (- (`self.K2_GetActorLocation` _ascharacter) (`SceneComponent.K2_GetComponentLocation` (`self.Left`)))) 500.0) true true))

(fn `RightLaunchPlayer`
  (params (Object :type "Object Object Reference"))
  (bind _ascharacter (cast `Character` Object))
  (`Character.LaunchCharacter` _ascharacter (* (`KismetMathLibrary.Normal` (- (`self.K2_GetActorLocation` _ascharacter) (`SceneComponent.K2_GetComponentLocation` (`self.Right`)))) 500.0) true true))

(fn `UserConstructionScript`)