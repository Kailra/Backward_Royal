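; BP_Dummy is a player character dummy assembled from modular skin meshes for head, hands, chest, legs and feet.
; Its construction script calls SetupModularMesh, which makes the main Mesh the leader pose component for each part, so all follow its animation.
; The main Mesh is hidden without propagating to children, leaving it as an invisible pose driver.
; The event graph holds only empty default events.
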(fn `SetupModularMesh`
  (bind _output_get (set `self.SkinArray` (`|MakeArray` (`self.Skin_Head`) (`self.Skin_Hand`) (`self.Skin_Chest`) (`self.Skin_Leg`) (`self.Skin_Foot`))))
  (for _array_element _output_get
    (`SkinnedMeshComponent.SetLeaderPoseComponent` _array_element (`self.Mesh`) false false)
    (`SceneComponent.SetVisibility` (`self.Mesh`) false false)))

(fn `UserConstructionScript`
  (`self.SetupModularMesh`))