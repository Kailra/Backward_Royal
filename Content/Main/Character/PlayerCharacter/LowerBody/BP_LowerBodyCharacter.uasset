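; BP_LowerBodyCharacter is a player character Blueprint that applies physical animation to part of its skeletal mesh.
; On BeginPlay it sets physical animation drives scaled from PAStrength below BodyName, simulates the bodies under that bone, then turns simulation back off from the head bone down.
; For testing only, key 1 toggles auto-run, which feeds forward movement input on Tick.
; Unconnected nodes that would exempt two further bones from simulation never run.
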(event `self.ReceiveBeginPlay`
  (bind _physicalanimation (`self.PhysicalAnimation`))
  (bind _body_name (`self.Body Name`))
  (bind _mesh (`self.Mesh`))
  (bind _pastrength (`self.PAStrength`))
  (bind _returnvalue (* _pastrength 1000.0))
  (bind _returnvalue_2 (* _pastrength 100.0))
  (`PhysicalAnimationComponent.SetSkeletalMeshComponent` _physicalanimation (`self.Mesh`))
  (`PhysicalAnimationComponent.ApplyPhysicalAnimationSettingsBelow` _physicalanimation _body_name (make `PhysicalAnimationData` true _returnvalue _returnvalue_2 _returnvalue _returnvalue_2) true)
  (`SkeletalMeshComponent.SetAllBodiesBelowSimulatePhysics` _mesh _body_name true false)
  (`SkeletalMeshComponent.SetAllBodiesBelowSimulatePhysics` _mesh (`self.head Bone Name`) false true))

(event `self.ReceiveTick`
  (params (DeltaSeconds :type "Float (single-precision)"))
  ; 테스트 전용
  ;; 키보드 1 < 자동 달리기>
  (if (`self.IsAutoRun`)
    (`self.AddMovementInput` (`self.GetActorForwardVector`))))

(event `Key|One`
  (params (Key :type "Key Structure"))
  ; 테스트 전용
  ;; 키보드 1 < 자동 달리기>
  (:`Pressed`
    (`/Engine/EditorBlueprintResources/StandardMacros.FlipFlop`
      (:`A`
        (set `self.IsAutoRun` true))
      (:`B`
        (set `self.IsAutoRun` false)))))

(fn `UserConstructionScript`)