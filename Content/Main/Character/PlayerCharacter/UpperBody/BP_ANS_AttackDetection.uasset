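; Anim notify state that marks the window in an animation during which a character's attack can detect hits.
; On begin it casts the mesh owner to BP_LowerBodyCharacter and enables attack detection on its AttackComponent.
; On end it disables detection the same way, leaving the detection logic itself to the component.
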(fn `Received_NotifyBegin`
  (params (MeshComp :type "SkeletalMeshComponent Object Reference") (Animation :type "AnimSequenceBase Object Reference") (TotalDuration :type "Float (single-precision)") (EventReference :type "AnimNotifyEventReference Structure (by ref)"))
  (returns (ReturnValue :type Boolean))
  (bind _asbp_lower_body_character (cast `/Game/Main/Character/PlayerCharacter/LowerBody/BP_LowerBodyCharacter` (`ActorComponent.GetOwner` MeshComp)))
  (`BRAttackComponent.SetAttackDetection` (`BaseCharacter.AttackComponent` _asbp_lower_body_character) true)
  (return false))

(fn `Received_NotifyEnd`
  (params (MeshComp :type "SkeletalMeshComponent Object Reference") (Animation :type "AnimSequenceBase Object Reference") (EventReference :type "AnimNotifyEventReference Structure (by ref)"))
  (returns (ReturnValue :type Boolean))
  (bind _asbp_lower_body_character (cast `/Game/Main/Character/PlayerCharacter/LowerBody/BP_LowerBodyCharacter` (`ActorComponent.GetOwner` MeshComp)))
  (`BRAttackComponent.SetAttackDetection` (`BaseCharacter.AttackComponent` _asbp_lower_body_character) false)
  (return false))