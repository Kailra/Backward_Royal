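; Game mode for a multiplayer game in which players control separate lower-body and upper-body pawns.
; On PostLogin it runs shared login handling, spawns a pawn at a player start and has the new controller possess it.
; If the BRPlayerState is not marked lower body, it calls a helper to attach the upper body to a lower body.
; An older two-player spawn-and-attach path using delayed retries remains but never runs.
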(event `self.K2_PostLogin`
  (params (NewPlayer :type "PlayerController Object Reference"))
  (`BRGameMode.HandlePlayerPostLogin` self NewPlayer)
  (bind _returnvalue (`BRGameMode.SpawnPawnForPlayer` self NewPlayer (`self.K2_FindPlayerStart` NewPlayer)))
  (`Controller.Possess` NewPlayer _returnvalue)
  (bind _asbrplayer_state (cast `BRPlayerState` (`Controller.PlayerState` NewPlayer)))
  (if (not (`BRPlayerState.GetIsLowerBody` _asbrplayer_state))
    (`BRGameMode.AttachUpperBodyToLowerBody` self (`self.NewVar`) NewPlayer)))

(fn `UserConstructionScript`)