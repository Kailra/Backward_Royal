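; A character Blueprint that appears to be a development test of physical animation on part of the body.
; On BeginPlay it applies physical animation below a configured bone and simulates physics on that bone's children, switching simulation back off for two exception chains and the head.
; For testing, key 1 toggles auto-run, which feeds forward movement input on Tick.
; An unarmed upper-body attack montage branch exists but is never executed.
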(event `self.ReceiveBeginPlay`
  (bind _physicalanimation_0 (`self.PhysicalAnimation_0`))
  (bind _body_name_0 (`self.Body Name_0`))
  (bind _mesh (`self.Mesh`))
  (`PhysicalAnimationComponent.SetSkeletalMeshComponent` _physicalanimation_0 (`self.Mesh`))
  (`PhysicalAnimationComponent.ApplyPhysicalAnimationSettingsBelow` _physicalanimation_0 _body_name_0 (make `PhysicalAnimationData` true 3000.0 300.0 3000.0 300.0) true)
  (`SkeletalMeshComponent.SetAllBodiesBelowSimulatePhysics` _mesh _body_name_0 true false)
  (`SkeletalMeshComponent.SetAllBodiesBelowSimulatePhysics` _mesh (`self.Except Bone Name1_0`) false true)
  (`SkeletalMeshComponent.SetAllBodiesBelowSimulatePhysics` _mesh (`self.Except Bone Name2_0`) false true)
  (`SkeletalMeshComponent.SetAllBodiesBelowSimulatePhysics` _mesh (`self.head Bone Name_0`) false true))

(event `self.ReceiveTick`
  (params (DeltaSeconds :type "Float (single-precision)"))
  ; 테스트 전용
  ;; 키보드 1 < 자동 달리기>
  (if (`self.IsAutoRun_0`)
    (`self.AddMovementInput` (`self.GetActorForwardVector`))))

(event `Key|One`
  (params (Key :type "Key Structure"))
  ; 테스트 전용
  ;; 키보드 1 < 자동 달리기>
  (:`Pressed`
    (`/Engine/EditorBlueprintResources/StandardMacros.FlipFlop`
      (:`A`
        (set `self.IsAutoRun_0` true))
      (:`B`
        (set `self.IsAutoRun_0` false)))))

(fn `UserConstructionScript`)