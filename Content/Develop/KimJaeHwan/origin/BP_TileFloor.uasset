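; BP_TileFloor is an actor that builds a rectangular floor out of repeated tile meshes.
; The construction script clears its Instanced Static Mesh component, then runs nested X and Y loops to add one local-space instance per grid cell, spaced by tile size.
; Tile counts and size are variables, and instancing serves the whole grid from one component.
; The event graph holds only disabled default events, so there is no runtime logic.
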(fn `UserConstructionScript`
  (`InstancedStaticMeshComponent.ClearInstances` (`self.InstancedStaticMesh`))
  (for _index (range (`self.TileCountX`))
    (for _index_2 (range (`self.TileCountY`))
      (`InstancedStaticMeshComponent.AddInstance` (`self.InstancedStaticMesh`) (`KismetMathLibrary.MakeTransform` (`KismetMathLibrary.MakeVector` (* _index (`self.TileSize`)) (* _index_2 (`self.TileSize`)))) false))))