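; Bridge obstacle actor that builds a randomized two-lane row of steps, with one real and one fake tile per step.
; On BeginPlay the server picks a random Seed, and OnRep_Seed rebuilds both instanced mesh components from a seeded stream, so every machine gets the same layout.
; Each step randomly puts the real tile left or right, adds a duplicate real tile high above it, and places the fake opposite.
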(event `self.ReceiveBeginPlay`
  (`/Engine/EditorBlueprintResources/ActorMacros.Switch Has Authority`
    (:`Authority`
      (set `self.Seed` (`KismetMathLibrary.RandomInteger` 999999)))))

(fn `OnRep_Seed`
  (`InstancedStaticMeshComponent.ClearInstances` (`self.ISMC_Fake`))
  (`InstancedStaticMeshComponent.ClearInstances` (`self.ISMC_Real`))
  (set `self.Stream` (`KismetMathLibrary.MakeRandomStream` (`self.Seed`)))
  (for _index (range 1 (+ (`self.StepCount`) 1))
    (if (`KismetMathLibrary.RandomBoolFromStream` (`self.Stream`))
      (`self.SetLeftReal` _index)
      (else
        (`self.SetRightReal` _index)))))

(fn `UserConstructionScript`)