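; Procedural rectangular fence actor that lays mesh instances along its perimeter in the construction script, sized by Width, Depth, Spacing and Offset.
; NewFunction0 builds the two X-axis sides and NewFunction the two rotated Y-axis sides, for both instanced mesh components.
; Only the first component is cleared before rebuilding.
; Inner loops ignore their index, so far-side instances stack as duplicates.
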(fn `NewFunction`
  (params (Target :type "InstancedStaticMeshComponent Object Reference"))
  (bind _spacing (`self.Spacing`))
  (bind _returnvalue (- (`KismetMathLibrary.FTrunc` (/ (`self.Depth`) _spacing)) 1))
  (for _index (range (+ _returnvalue 1))
    (bind _returnvalue_2 (+ (* _index _spacing) (`self.Offset`)))
    (`InstancedStaticMeshComponent.AddInstance` Target (`KismetMathLibrary.MakeTransform` (`KismetMathLibrary.MakeVector` 0.0 _returnvalue_2) (struct :`Yaw` 90.0)) false)
    (for _index_2 (range (+ _returnvalue 1))
      (`InstancedStaticMeshComponent.AddInstance` Target (`KismetMathLibrary.MakeTransform` (`KismetMathLibrary.MakeVector` (`self.Width`) _returnvalue_2) (struct :`Yaw` 90.0)) false))))

(fn `NewFunction_0`
  (params (Target :type "InstancedStaticMeshComponent Object Reference"))
  (bind _spacing (`self.Spacing`))
  (bind _returnvalue (- (`KismetMathLibrary.FTrunc` (/ (`self.Width`) _spacing)) 1))
  (for _index (range (+ _returnvalue 1))
    (`KismetArrayLibrary.Array_Add` (`self.Index`) _index)
    (bind _returnvalue_2 (+ (* _index _spacing) (`self.Offset`)))
    (`InstancedStaticMeshComponent.AddInstance` Target (`KismetMathLibrary.MakeTransform` (`KismetMathLibrary.MakeVector` _returnvalue_2)) false)
    (for _index_2 (range (+ _returnvalue 1))
      (`InstancedStaticMeshComponent.AddInstance` Target (`KismetMathLibrary.MakeTransform` (`KismetMathLibrary.MakeVector` _returnvalue_2 (`self.Depth`))) false))))

(fn `UserConstructionScript`
  (bind _instancedstaticmesh1 (`self.InstancedStaticMesh1`))
  (bind _instancedstaticmesh (`self.InstancedStaticMesh`))
  (`InstancedStaticMeshComponent.ClearInstances` (`self.InstancedStaticMesh`))
  (`self.NewFunction_0` _instancedstaticmesh)
  (`self.NewFunction` _instancedstaticmesh)
  (`self.NewFunction_0` _instancedstaticmesh1)
  (`self.NewFunction` _instancedstaticmesh1))