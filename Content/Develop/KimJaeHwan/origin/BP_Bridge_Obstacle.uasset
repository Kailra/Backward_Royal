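; BP_Bridge_Obstacle is a bridge obstacle that lays out a random path of paired real and fake steps.
; On BeginPlay it clears both instanced mesh components, then picks the left or right side as real for each step.
; SetLeftReal and SetRightReal place instances along X at mirrored Y offsets, with the fake opposite the real one.
; Each real step also gets a duplicate high above it in the real component.
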(event `self.ReceiveBeginPlay`
  (`InstancedStaticMeshComponent.ClearInstances` (`self.ISMC_Fake`))
  (`InstancedStaticMeshComponent.ClearInstances` (`self.ISMC_Real`))
  (for _index (range 1 (+ (`self.StepCount`) 1))
    (if (`KismetMathLibrary.RandomBool`)
      (`self.SetLeftReal` _index)
      (else
        (`self.SetRightReal` _index)))))

(fn `UserConstructionScript`)