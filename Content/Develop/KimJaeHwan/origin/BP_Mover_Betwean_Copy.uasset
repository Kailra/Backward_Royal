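; A mover Blueprint that eases a target component back and forth between Start and End offsets from its starting world location.
; BeginPlay records the target's initial location after running the parent logic.
; Each OnUpdate sets the location from an Ease of GetAlpha with configurable function and exponent, without sweep.
; OnPeriodEnd swaps Start and End, reversing the direction for the next period.
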(event `self.ReceiveBeginPlay`
  (`parent.ReceiveBeginPlay`)
  (set `self.InitialLocation` (`self.K2_GetComponentLocation` (`self.Target`))))

(event `self.OnUpdate`
  (`self.K2_SetWorldLocation` (`self.Target`) (+ (`|EaseFunction` (`self.Function`) (`self.GetAlpha`) (`self.Start`) (`self.End`) (`self.Exponent`)) (`self.InitialLocation`)) false false))

(event `self.OnPeriodEnd`
  (`/Game/Asset/Maps/Platformer_8_Underworld/Blueprints/Components/BML_Platformer.Swap` (`self.Start`) (`self.End`)))