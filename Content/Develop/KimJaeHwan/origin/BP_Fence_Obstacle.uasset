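; BP_Fence_Obstacle is an obstacle actor that builds rows of fence pieces, each with one randomly placed gap.
; On BeginPlay it loops over RowCount rows, picks a random hole index per row, and skips that slot.
; All other slots become rotated instances on an InstancedStaticMesh, spaced by RowDistance along X and FenceWidth along Y.
; The layout is generated at runtime only, since the construction script is empty.
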(event `self.ReceiveBeginPlay`
  (for _index (range 1 (+ (`self.RowCount`) 1))
    (bind _output_get (set `self.HoleIndex` (`KismetMathLibrary.RandomIntegerInRange` 1 (`self.FenceCount`))))
    (for _index_2 (range 1 (+ (`self.FenceCount`) 1))
      (if (not (== _index_2 _output_get))
        (`InstancedStaticMeshComponent.AddInstance` (`self.InstancedStaticMesh`) (`KismetMathLibrary.MakeTransform` (`KismetMathLibrary.MakeVector` (* _index (`self.RowDistance`)) (* _index_2 (`self.FenceWidth`))) (struct :`Yaw` 90.0)) false)))))

(fn `UserConstructionScript`)