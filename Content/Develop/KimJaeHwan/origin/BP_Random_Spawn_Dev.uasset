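; BP_Random_Spawn_Dev scatters instanced meshes over a jittered grid and supplies their positions to BP_ItemSpawner_Dev.
; On BeginPlay, the server fills the width-by-depth area with randomly offset, random-yaw instances, storing each transform in ActorTransforms.
; It converts those transforms to world space, raises and rolls them, then appends them to the spawner's ExternalTransforms.
; An OnRep on ActorTransforms rebuilds the instances from the replicated array.
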(event `self.ReceiveBeginPlay`
  (`/Engine/EditorBlueprintResources/ActorMacros.Switch Has Authority`
    (:`Authority`
      (`InstancedStaticMeshComponent.ClearInstances` (`self.InstancedStaticMesh`))
      (`self.RandomSpawn`))))

(fn `OnRep_ActorTransforms`
  (`InstancedStaticMeshComponent.ClearInstances` (`self.InstancedStaticMesh`))
  (for _array_element (`self.ActorTransforms`)
    (`InstancedStaticMeshComponent.AddInstance` (`self.InstancedStaticMesh`) _array_element false)))

(fn `RandomSpawn`
  (bind _jitteramount (`self.JitterAmount`))
  (bind _actortransforms (`self.ActorTransforms`))
  (bind _returnvalue (`KismetMathLibrary.RandomFloatInRange` (- _jitteramount (* _jitteramount 2.0)) (`self.JitterAmount`)))
  (for _index (range (+ (`KismetMathLibrary.FTrunc` (/ (`self.Width`) (`self.GridSpacing`))) 1))
    (for _index_2 (range (+ (`KismetMathLibrary.FTrunc` (/ (`self.Depth`) (`self.GridSpacing`))) 1))
      (`KismetArrayLibrary.Array_Add` _actortransforms (`KismetMathLibrary.MakeTransform` (`KismetMathLibrary.MakeVector` (+ (* _index (`self.GridSpacing`)) _returnvalue) (+ (* _index_2 (`self.GridSpacing`)) _returnvalue)) (`KismetMathLibrary.MakeRotator` 0.0 0.0 (`KismetMathLibrary.RandomFloatInRange` 0.0 360.0))))
      (`InstancedStaticMeshComponent.AddInstance` (`self.InstancedStaticMesh`) (`|GetArrayItem` _actortransforms (`self.TransfoemsIndexNum`)) false)
      (set `self.TransfoemsIndexNum` (+ (`self.TransfoemsIndexNum`) 1))))
  (bind _returnvalue_2 (`GameplayStatics.GetActorOfClass` "/Game/Develop/KimJaeHwan/origin/BP_ItemSpawner_Dev.BP_ItemSpawner_Dev_C"))
  (for _array_element (`self.ActorTransforms`)
    (bind _returnvalue_3 (`KismetMathLibrary.ComposeTransforms` _array_element (`self.GetTransform`)))
    (`KismetArrayLibrary.Array_Add` (`/Game/Develop/KimJaeHwan/origin/BP_ItemSpawner_Dev.ExternalTransforms` _returnvalue_2) (`KismetMathLibrary.MakeTransform` (+ (.location _returnvalue_3) (0.0 0.0 50.0)) (`KismetMathLibrary.MakeRotator` (+ (.roll (.rotation _returnvalue_3)) 90.0) (.pitch (.rotation _returnvalue_3)) (.yaw (.rotation _returnvalue_3))) (.scale _returnvalue_3)))))

(fn `UserConstructionScript`)