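; AI enemy character Blueprint that wanders randomly with physics-driven wobble on its body.
; On authority, BeginPlay applies physical animation, simulates bodies below a chosen bone, and starts looping AIMoveTo calls to random reachable points.
; Damage only prints the instigator's team number and a win message at zero HP; key 1 toggles test auto-run.
; Bush-mask material parameter updates exist, but their timer setup is disconnected.
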(event `self.ReceiveBeginPlay`
  (bind _physicalanimation (`self.PhysicalAnimation`))
  (bind _body_name (`self.Body Name`))
  (bind _pastrength (`self.PAStrength`))
  (bind _returnvalue (* _pastrength 1000.0))
  (bind _returnvalue_2 (* _pastrength 100.0))
  (`/Engine/EditorBlueprintResources/ActorMacros.Switch Has Authority`
    (:`Authority`
      (`PhysicalAnimationComponent.SetSkeletalMeshComponent` _physicalanimation (`self.Mesh`))
      (`PhysicalAnimationComponent.ApplyPhysicalAnimationSettingsBelow` _physicalanimation _body_name (make `PhysicalAnimationData` true _returnvalue _returnvalue_2 _returnvalue _returnvalue_2) true)
      (`SkeletalMeshComponent.SetAllBodiesBelowSimulatePhysics` (`self.Mesh`) _body_name true false)
      (`self.MoveToRandomLocation`))))

(event `UpdateBushMask`
  (`self.UpdateBushMaskLocation`))

(event `MoveToRandomLocation`
  (`|AIMoveTo` self (`NavigationSystemV1.K2_GetRandomReachablePointInRadius` (`self.K2_GetActorLocation`) 1500.0 null null) null
    (:`OnSuccess`
      _)
    (:`OnFail`
      _))
  (`KismetSystemLibrary.Delay` 1.0)
  (`self.MoveToRandomLocation`))

(event `self.ReceiveTick`
  (params (DeltaSeconds :type "Float (single-precision)"))
  ; 테스트 전용
  ;; 키보드 1 < 자동 달리기>
  (if (`self.IsAutoRun`)
    (`self.AddMovementInput` (`self.GetActorForwardVector`))))

(event `Key|One`
  (params (Key :type "Key Structure"))
  ; 테스트 전용
  ;; 키보드 1 < 자동 달리기>
  (:`Pressed`
    (`/Engine/EditorBlueprintResources/StandardMacros.FlipFlop`
      (:`A`
        (set `self.IsAutoRun` true))
      (:`B`
        (set `self.IsAutoRun` false)))))

(event `self.ReceiveAnyDamage`
  (params (Damage :type "Float (single-precision)") (DamageType :type "DamageType Object Reference") (InstigatedBy :type "Controller Object Reference") (DamageCauser :type "Actor Object Reference"))
  (bind _asbrplayer_state (cast `BRPlayerState` (`Controller.PlayerState` InstigatedBy)))
  (`KismetSystemLibrary.PrintString` (`KismetStringLibrary.Conv_IntToString` (`BRPlayerState.TeamNumber` _asbrplayer_state)))
  (if (<= (`self.CurrentHP`) 0.0)
    (`KismetSystemLibrary.PrintString` "우승")))

(fn `UserConstructionScript`)