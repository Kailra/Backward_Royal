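; A temporary character Blueprint that tests physical animation on part of the skeleton alongside a weight-scaled attack montage.
; On BeginPlay it applies strong physical animation drives below a chosen bone and simulates physics on the bodies beneath it, switching simulation back off for two excepted bone chains.
; A trigger event plays a horizontal attack montage at a rate that drops as the current weapon's mass rises relative to its attack speed coefficient.
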(event `self.ReceiveBeginPlay`
  (bind _physicalanimation (`self.PhysicalAnimation`))
  (bind _body_name (`self.Body Name`))
  (bind _mesh (`self.Mesh`))
  (`PhysicalAnimationComponent.SetSkeletalMeshComponent` _physicalanimation (`self.Mesh`))
  (`PhysicalAnimationComponent.ApplyPhysicalAnimationSettingsBelow` _physicalanimation _body_name (make `PhysicalAnimationData` true 3000.0 300.0 3000.0 300.0) true)
  (`SkeletalMeshComponent.SetAllBodiesBelowSimulatePhysics` _mesh _body_name true false)
  (`SkeletalMeshComponent.SetAllBodiesBelowSimulatePhysics` _mesh (`self.Except Bone Name1`) false true)
  (`SkeletalMeshComponent.SetAllBodiesBelowSimulatePhysics` _mesh (`self.Except Bone Name2`) false true))

(event `self.TriggerUpperBodyAttack`
  (bind _currentweapon (`self.CurrentWeapon`))
  (bind (_weaponstats_weaponmesh _weaponstats_basedamage _weaponstats_masskg) (break `WeaponData` (`BaseWeapon.WeaponStats` _currentweapon)))
  (`|PlayMontage` (`self.Mesh`) "/Game/Asset/Animations/Two_Handed_Sword/Animations/Sequence_UE5/02_Attack/10_Combo_Attack_Still_01/AS_Horizontal_Attack_Montage.AS_Horizontal_Attack_Montage" (/ 1.0 (/ _weaponstats_masskg (`BaseWeapon.AttackSpeedCoefficient` _currentweapon)))))

(fn `UserConstructionScript`)