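; BP_TestGameMode is a test game mode that lets two players share one body, with the second player joining as the upper body.
; On the second PostLogin, it waits briefly, polls until that player has a valid pawn, then destroys it.
; It spawns and possesses a BP_UpperBodyPawn, then snaps it to the HeadMountPoint of player 0's BP_LowerBodyCharacter.
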(event `self.K2_PostLogin`
  (params (NewPlayer :type "PlayerController Object Reference"))
  (bind _returnvalue (`Controller.K2_GetPawn` NewPlayer))
  ;[1 1 1] 2플레이어 기본 몸통 삭제
  (bind _returnvalue_2 (`self.GetNumPlayers`))
  (switch `int` _returnvalue_2
    (:`2`
      (`KismetSystemLibrary.Delay` 0.2)
      (`/Engine/EditorBlueprintResources/StandardMacros.IsValid` _returnvalue :!label _label
        (:`Is Valid`
          ;[1 1 1] 머리 생성 빙의
          (`self.K2_DestroyActor` _returnvalue)
          (bind _returnvalue_3 (`|SpawnActorFromClass` "/Game/Main/Character/PlayerCharacter/UpperBody/BP_UpperBodyPawn.BP_UpperBodyPawn_C" (`KismetMathLibrary.MakeTransform` (0.0 0.0 0.0)) "Undefined" "MultiplyWithRoot" null null))
          (`Controller.Possess` NewPlayer _returnvalue_3)
          ;[1 1 1] 몸통 찾아서 연결
          (bind _asbp_lower_body_character (cast `/Game/Main/Character/PlayerCharacter/LowerBody/BP_LowerBodyCharacter` (`GameplayStatics.GetPlayerPawn` 0)))
          (`self.K2_AttachToComponent` _returnvalue_3 (`PlayerCharacter.HeadMountPoint` _asbp_lower_body_character) "None" "SnapToTarget" "SnapToTarget" "SnapToTarget" true))
        (:`Is Not Valid`
          (`KismetSystemLibrary.Delay` 0.1)
          (goto _label))))))

(fn `UserConstructionScript`)