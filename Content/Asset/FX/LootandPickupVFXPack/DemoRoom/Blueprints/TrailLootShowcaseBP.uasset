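; Demo showcase actor for a loot drop: a projectile sphere with a trail that lands, displays loot effects, then plays a pickup effect and expires.
; The construction script picks one random index to set matching Niagara effects and sphere material from parallel arrays.
; Tick keeps the pillar, glow and activation effects on the moving sphere.
; The first sphere hit triggers pillar and glow, then a timed shutdown, pickup burst and lifespan.
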(event `self.ReceiveBeginPlay`
  (`ActorComponent.Activate` (`self.ProjectileMovement`) false)
  (`ActorComponent.Activate` (`self.NS_Trail`) false)
  (`KismetSystemLibrary.Delay` (`KismetMathLibrary.RandomFloatInRange` 0.2 1.0))
  (`ActorComponent.Activate` (`self.NS_Activation`) true))

(event `self.ReceiveTick`
  (params (DeltaSeconds :type "Float (single-precision)"))
  (`SceneComponent.K2_SetWorldLocation` (`self.NS_LightPillarVFX`) (`SceneComponent.K2_GetComponentLocation` (`self.SphereMesh`)) false false)
  (`SceneComponent.K2_SetWorldLocation` (`self.NS_GlowVFX`) (`SceneComponent.K2_GetComponentLocation` (`self.SphereMesh`)) false false)
  (`SceneComponent.K2_SetWorldLocation` (`self.NS_Activation`) (`SceneComponent.K2_GetComponentLocation` (`self.SphereMesh`)) false false))

(event `self.RootSphere.OnComponentHit`
  (params (HitComponent :type "PrimitiveComponent Object Reference") (OtherActor :type "Actor Object Reference") (OtherComp :type "PrimitiveComponent Object Reference") (NormalImpulse :type "Vector Structure") (Hit :type "HitResult Structure (by ref)"))
  (`/Engine/EditorBlueprintResources/StandardMacros.DoOnce` false :!label _label
    (:`Completed`
      (`ActorComponent.Activate` (`self.NS_LightPillarVFX`) true)
      (`ActorComponent.Activate` (`self.NS_GlowVFX`) true)
      (`KismetSystemLibrary.Delay` 3.0)
      (`ActorComponent.Deactivate` (`self.NS_Trail`))
      (`KismetSystemLibrary.Delay` 2.0)
      (`ActorComponent.Deactivate` (`self.NS_GlowVFX`))
      (`ActorComponent.Deactivate` (`self.NS_LightPillarVFX`))
      (`ActorComponent.Deactivate` (`self.NS_Trail`))
      (`SceneComponent.SetVisibility` (`self.NS_LightPillarVFX`) false false)
      (`SceneComponent.SetVisibility` (`self.NS_GlowVFX`) false false)
      (`SceneComponent.SetVisibility` (`self.NS_Trail`) false false)
      (`ActorComponent.Activate` (`self.NS_PickupVFX`) true)
      (`SceneComponent.SetVisibility` (`self.SphereMesh`) false false)
      (`SceneComponent.SetVisibility` (`self.RootSphere`) false false)
      (`self.SetLifeSpan` 3.0))))

(event `self.SphereMesh.OnComponentHit`
  (params (HitComponent :type "PrimitiveComponent Object Reference") (OtherActor :type "Actor Object Reference") (OtherComp :type "PrimitiveComponent Object Reference") (NormalImpulse :type "Vector Structure") (Hit :type "HitResult Structure (by ref)"))
  (goto _label))

(fn `UserConstructionScript`
  (bind _index (`self.Index`))
  (bind _output_get (set `self.Index` (`KismetMathLibrary.RandomIntegerInRange` 0 8)))
  (`NiagaraComponent.SetAsset` (`self.NS_LightPillarVFX`) (`|GetArrayItem` (`self.LightPillarVFXArray`) _output_get) true)
  (`NiagaraComponent.SetAsset` (`self.NS_GlowVFX`) (`|GetArrayItem` (`self.GlowVFXArray`) _output_get) true)
  (`NiagaraComponent.SetAsset` (`self.NS_Activation`) (`|GetArrayItem` (`self.ActivationVFXArray`) _output_get) true)
  (`PrimitiveComponent.SetMaterial` (`self.SphereMesh`) 0 (`|GetArrayItem` (`self.SphereMaterialArray`) (`self.Index`)))
  (`NiagaraComponent.SetAsset` (`self.NS_PickupVFX`) (`|GetArrayItem` (`self.PickupVFXarray`) _index) true)
  (`NiagaraComponent.SetAsset` (`self.NS_Trail`) (`|GetArrayItem` (`self.TrailVFXArray`) _index) true))